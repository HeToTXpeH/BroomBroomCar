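; Player controller that owns the local HUD and menu widgets.
; On BeginPlay it creates the tab scoreboard and fast menu for clients and the listen-server host, with a start screen for the host only.
; Possessing a BP_Buggy shows W_Bar; other pawns hide it.
; Escape or Delete toggles the fast menu, held Score shows refreshed stats except when spectating, and addrotator offsets control pitch.
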(event `Event add rotator`
  (params (Rotator :type "Float (double-precision)"))
  (`self.SetControlRotation` (`KismetMathLibrary.MakeRotator` (.roll (`self.GetControlRotation`)) (+ (.pitch (`self.GetControlRotation`)) Rotator) (.yaw (`self.GetControlRotation`)))))

(event `self.ReceivePossess`
  (params (PossessedPawn :type "Pawn Object Reference"))
  (cast `/Game/Blueprints/BP_Buggy` PossessedPawn
    (:`then`
      (`self.EventRemoveWidgets` true))
    (:`CastFailed`
      (`self.EventRemoveWidgets` false))))

(event `EventRemoveWidgets`
  (params (Remove :type Boolean))
  (if Remove
    (`/Engine/EditorBlueprintResources/StandardMacros.IsValid` (`self.W_Bar`)
      (:`Is Valid`
        _)
      (:`Is Not Valid`
        (bind _returnvalue (`|CreateWidget` "/Game/Widgets/InGameHUD/W_Bar.W_Bar_C" self))
        (set `self.W_Bar` _returnvalue)))
    (`UserWidget.AddToViewport` (`self.W_Bar`) 0)
    (else
      (`/Engine/EditorBlueprintResources/StandardMacros.IsValid` (`self.W_Bar`)
        (:`Is Valid`
          (`Widget.RemoveFromParent` (`self.W_Bar`)))))))

(event `self.ReceiveBeginPlay`
  (if (`KismetSystemLibrary.IsDedicatedServer`)
    _
    (elif (`KismetSystemLibrary.IsServer`)
      (if (== (`GameplayStatics.GetPlayerController` 0) self)
        (`|ExecutionSequence`
          (:`then_0`
            (bind _returnvalue (`|CreateWidget` "/Game/Widgets/W_Tab.W_Tab_C" self :!label _label))
            (set `self.W_TabMenu` _returnvalue)
            (bind _returnvalue_2 (`|CreateWidget` "/Game/Widgets/W_FastMenu.W_FastMenu_C" self))
            (set `self.W_Menu` _returnvalue_2))
          (:`then_1`
            (bind _returnvalue_3 (`|CreateWidget` "/Game/Widgets/W_Start.W_Start_C" self))
            (`UserWidget.AddToViewport` _returnvalue_3 0))))
      (else
        (goto _label)))))

(event `Key|Escape`
  (params (Key :type "Key Structure"))
  (:`Pressed`
    (`/Game/Widgets/W_FastMenu.Swap widget` (`self.W_Menu`) :!label _label_2)))

(event `Key|Delete`
  (params (Key :type "Key Structure"))
  (:`Pressed`
    (goto _label_2)))

(event `InputAction|Score`
  (params (Key :type "Key Structure"))
  (bind _returnvalue (`self.K2_GetPawn`))
  (bind _w_tabmenu (`self.W_TabMenu`))
  (:`Pressed`
    (cast `/Game/Blueprints/GameStatus/BP_SpectratorPawn` _returnvalue
      (:`CastFailed`
        (`UserWidget.AddToViewport` _w_tabmenu 0)
        (`/Game/Widgets/W_Tab.refreshPlayerStats` _w_tabmenu))))
  (:`Released`
    (cast `/Game/Blueprints/GameStatus/BP_SpectratorPawn` _returnvalue
      (:`CastFailed`
        (`Widget.RemoveFromParent` _w_tabmenu)))))

(fn `UserConstructionScript`)