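; Default game mode that starts the match on BeginPlay by calling StartMatch on BP_DefautGameStats, the game state.
; ToSpectrator spawns a spectator pawn at the point stored by SetMapDefauts, possesses it with the player's controller and destroys the old character.
; ChangeMap builds a ServerTravel console command from a map name, with no separating space.
; StopMatch and PlayerFinish are stubs, the latter holding an unconnected spectator call.
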(event `self.ReceiveBeginPlay`
  (`self.StartMatch`))

(fn `ChangeMap`
  (params (Map :type String))
  (`KismetSystemLibrary.ExecuteConsoleCommand` (`KismetStringLibrary.Concat_StrStr` "ServerTravel " Map) null))

(fn `PlayerFinish`
  (params (Character :type "Pawn Object Reference") (Controller :type "PlayerController Object Reference")))

(fn `SetMapDefauts`
  (params (SpectratorPoint :type "TargetPoint Object Reference"))
  (set `self.SpectratorPoint` SpectratorPoint))

(fn `StartMatch`
  (bind _asbp_deathmatch_game_stats (cast `/Game/Blueprints/GameStatus/BP_DefautGameStats` (`GameplayStatics.GetGameState`)))
  (`/Game/Blueprints/GameStatus/BP_DefautGameStats.StartMatch` _asbp_deathmatch_game_stats))

(fn `StopMatch`)

(fn `ToSpectrator`
  (params (Controller :type "Controller Object Reference") (Character :type "/Game/Blueprints/Character/BP_PlayerCharacter Object Reference"))
  (bind _returnvalue (`|SpawnActorFromClass` "/Game/Blueprints/GameStatus/BP_SpectratorPawn.BP_SpectratorPawn_C" (`self.GetTransform` (`self.SpectratorPoint`)) "Undefined" "OverrideRootScale" Controller Character))
  (`Controller.Possess` Controller _returnvalue)
  (`/Engine/EditorBlueprintResources/StandardMacros.IsValid` Character
    (:`Is Valid`
      (`self.K2_DestroyActor` Character))))

(fn `UserConstructionScript`)